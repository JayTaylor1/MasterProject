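; Boss laser actor that fires a green Niagara beam which gradually swings toward the player and damages them on contact.
; Each Tick lerps and normalises the aim vector toward the player at BeamSpeed, independent of delta time.
; A box trace sized from BeamWidth follows that aim to just beyond player distance.
; Hits set the beam length and damage a Player every frame; misses draw the beam past player distance.
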(event `self.ReceiveTick`
  (params (DeltaSeconds :type "Float (single-precision)"))
  (bind _returnvalue (/ (`self.BeamWidth`) 4.0))
  (`self.CreateTarget`)
  (bind (_outhit _returnvalue_2) (`KismetSystemLibrary.BoxTraceSingle` (`SceneComponent.K2_GetComponentLocation` (`self.Niagara`)) (+ (`SceneComponent.K2_GetComponentLocation` (`self.Niagara`)) (* (`self.TargetVector`) (+ (`KismetMathLibrary.Vector_Distance` (`SceneComponent.K2_GetComponentLocation` (`self.Niagara`)) (`self.K2_GetActorLocation` (`GameplayStatics.GetPlayerCharacter` 0))) (`self.BeamSizeBonus`)))) (`KismetMathLibrary.MakeVector` _returnvalue _returnvalue _returnvalue) (struct) "TraceTypeQuery1"))
  (if _returnvalue_2
    (bind (_bblockinghit _binitialoverlap _time _distance _location _impactpoint _normal _impactnormal _physmat _hitactor) (`GameplayStatics.BreakHitResult` _outhit))
    ;[1 1 1] CollidedLazerMovement
    (`FXSystemComponent.SetVectorParameter` (`self.Niagara`) "LaserTarget" (* (`self.TargetVector`) (+ _distance (`self.BeamSizeBonus`))))
    ;;[1 1 1] Player Damage from laser
    (bind _asplayer (cast `/Game/BloodRift/Character/Player` _hitactor))
    (`/Game/BloodRift/Character/Player.TakeDamage` _asplayer (`self.BeamDammage`))
    (else
      ;[1 1 1] NonColideLazerMovement
      (`FXSystemComponent.SetVectorParameter` (`self.Niagara`) "LaserTarget" (* (`self.TargetVector`) (+ (`KismetMathLibrary.Vector_Distance` (`SceneComponent.K2_GetComponentLocation` (`self.Niagara`)) (`self.K2_GetActorLocation` (`GameplayStatics.GetPlayerCharacter` 0))) (`self.BeamSizeBonus`)))))))

(event `self.ReceiveBeginPlay`
  (bind _niagara (`self.Niagara`))
  ;[1 1 1] LazerInitialization
  (set `self.TargetVector` (* (`SceneComponent.GetForwardVector` (`self.Cube`)) (`self.BeamSizeBonus`)))
  (`FXSystemComponent.SetFloatParameter` _niagara "LaserWidth" (`self.BeamWidth`))
  (`FXSystemComponent.SetColorParameter` _niagara "LaserColor" (struct :`G` 0.17 :`A` 1.0)))

(fn `CreateTarget`
  (set `self.TargetVector` (`KismetMathLibrary.Normal` (`KismetMathLibrary.VLerp` (`self.TargetVector`) (`KismetMathLibrary.Conv_RotatorToVector` (`KismetMathLibrary.FindLookAtRotation` (`SceneComponent.K2_GetComponentLocation` (`self.Niagara`)) (`SceneComponent.K2_GetComponentLocation` (`Character.CapsuleComponent` (`GameplayStatics.GetPlayerCharacter` 0))))) (`self.BeamSpeed`)))))

(fn `UserConstructionScript`)