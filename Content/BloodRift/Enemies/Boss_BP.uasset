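; Boss enemy that loops between two homing-projectile attacks, a timed stream or delayed radial waves, picked at random.
; BeginPlay precomputes the ring of rotations, which Tick cycles through to turn the stream's spawn point.
; Below a health threshold, it stops attacking once, raises damage resistance and spawns two ranged-enemy portals at spawn-point arrows near the player.
; Tick resumes attacks and resets resistance when no Enemy-tagged actors remain.
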(event `self.ReceiveBeginPlay`
  (bind (_current_rotation_roll _current_rotation_pitch) (`KismetMathLibrary.BreakRotator` (`self.Current_Rotation`)))
  (bind _homing_number_multi (`self.Homing_Number_Multi`))
  (for _ (range _homing_number_multi)
    (bind _output_get (set `self.Current_Rotation` (`KismetMathLibrary.MakeRotator` 0.0 (+ (/ 360.0 (`KismetMathLibrary.Conv_IntToDouble` _homing_number_multi)) _current_rotation_pitch) 90.0)))
    (`KismetArrayLibrary.Array_Add` (`self.Homing_Spawn_Rotations_Multi`) _output_get))
  (`self.Choose_Moves`))

(event `self.ReceiveTick`
  (params (DeltaSeconds :type "Float (single-precision)"))
  (bind _homing_spawn_rotations_multi (`self.Homing_Spawn_Rotations_Multi`))
  (bind _current_rotation_number (`self.Current_Rotation_Number`))
  (`|ExecutionSequence`
    (:`then_0`
      (`KismetSystemLibrary.Delay` (/ (`self.Homing_Duration_Single`) (`KismetMathLibrary.Conv_IntToDouble` (`self.Homing_Number_Single`))))
      (`SceneComponent.K2_SetWorldRotation` (`self.HomingSPawn`) (`|GetArrayItem` _homing_spawn_rotations_multi (`self.Current_Rotation_Number`)) false false)
      (`/Engine/EditorBlueprintResources/StandardMacros.IncrementInt` _current_rotation_number
        (:`  `
          (if (== (`KismetArrayLibrary.Array_Length` _homing_spawn_rotations_multi) _current_rotation_number)
            (set `self.Current_Rotation_Number` 0)))))
    (:`then_1`
      (bind _outactors (`GameplayStatics.GetAllActorsWithTag` "Enemy"))
      (if (== (`KismetArrayLibrary.Array_Length` _outactors) 0)
        (`/Engine/EditorBlueprintResources/StandardMacros.DoOnce` false :!label _label
          (:`Completed`
            (`self.Choose_Moves`)
            (set `self.Damage_Resistance` 50.0)))
        (else
          (`/Engine/EditorBlueprintResources/StandardMacros.DoOnce` false
            (:`Completed`
              (goto _label :!via `Reset`))))))))

(event `Choose_Moves`
  (if (`self.Dead?`)
    _
    (elif (`self.Can_Invincible?`)
      (if (< (`self.Health`) 60.0)
        (`/Engine/EditorBlueprintResources/StandardMacros.DoOnce` false
          (:`Completed`
            (`self.Spawn_Enemies`)
            (set `self.Can_Invincible?` false)
            (set `self.Damage_Resistance` 100.0)))
        (else
          (switch `int` (`KismetMathLibrary.RandomIntegerInRange` 0 1) :!label _label_2
            (:`0`
              (set `self.Spawn_Homing?` true)
              (`self.Homing_Attack`))
            (:`1`
              (`self.Multi_Homing`)))))
      (else
        (goto _label_2)))))

(event `Homing_Attack`
  (bind _homingspawn (`self.HomingSPawn`))
  (bind (_returnvalue_roll _returnvalue_pitch _returnvalue_yaw) (`KismetMathLibrary.BreakRotator` (`SceneComponent.K2_GetComponentRotation` _homingspawn)))
  (`|ExecutionSequence`
    (:`then_0`
      (`KismetSystemLibrary.Delay` (`self.Homing_Duration_Single`))
      (set `self.Spawn_Homing?` false)
      (`KismetSystemLibrary.Delay` 2.0)
      (`self.Choose_Moves`))
    (:`then_1`
      (if (`self.Spawn_Homing?`) :!label _label_3
        (`KismetSystemLibrary.Delay` (/ (`self.Homing_Duration_Single`) (`KismetMathLibrary.Conv_IntToDouble` (`self.Homing_Number_Single`))))
        (`|SpawnActorFromClass` "/Game/BloodRift/Enemies/Homing_BP.Homing_BP_C" (`KismetMathLibrary.MakeTransform` (`SceneComponent.K2_GetComponentLocation` _homingspawn) (`KismetMathLibrary.MakeRotator` _returnvalue_roll _returnvalue_pitch _returnvalue_yaw)) "Undefined" "OverrideRootScale" null null)
        (goto _label_3)))))

(event `Spawn_Enemies`
  ;[1 1 1] Ranged
  (`|ExecutionSequence`
    (:`then_1`
      (for _ (range 2)
        (bind _outactors (`GameplayStatics.GetAllActorsOfClass` null))
        (bind _outitem (`KismetArrayLibrary.Array_Random` (`self.GetComponentsByTag` (`.ReturnValue` (`GameplayStatics.FindNearestActor` (`SceneComponent.K2_GetComponentLocation` (`Character.Mesh` (`GameplayStatics.GetPlayerCharacter` 0))) _outactors)) "/Script/Engine.ArrowComponent" "Spawn_Point")))
        (`|SpawnActorFromClass` "/Game/BloodRift/Enemies/Portal_Ranged_BP.Portal_Ranged_BP_C" (`KismetMathLibrary.MakeTransform` (`SceneComponent.K2_GetComponentLocation` _outitem)) "Undefined" "OverrideRootScale" null null)
        (`ActorComponent.K2_DestroyComponent` _outitem)))))

(event `Multi_Homing`
  (for _index (range (`self.Multi_Circles`))
    (for _index_2 (range (`self.Homing_Number_Multi`))
      (bind _returnvalue (`|SpawnActorFromClass` "/Game/BloodRift/Enemies/Homing_BP.Homing_BP_C" (`KismetMathLibrary.MakeTransform` (`SceneComponent.K2_GetComponentLocation` (`self.HomingSPawn`)) (`|GetArrayItem` (`self.Homing_Spawn_Rotations_Multi`) _index_2)) "Undefined" "OverrideRootScale" null null))
      (set `/Game/BloodRift/Enemies/Homing_BP.Fly_Speed` 0.03 _returnvalue)
      (set `/Game/BloodRift/Enemies/Homing_BP.Delay` (* 0.2 (`KismetMathLibrary.Conv_IntToDouble` (+ _index 1))) _returnvalue)))
  (`KismetSystemLibrary.Delay` 2.0)
  (`self.Choose_Moves`))

(fn `UserConstructionScript`
  (`parent.UserConstructionScript`))