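; Parent enemy Blueprint for BloodRift that handles taking damage across three health phases.
; Take_Damage applies percentage resistance, adding a critical multiplier only when a fully charged attack hits the "Crit" collider.
; Depleted health advances the phase and refills from that stage's health, or marks the enemy dead in phase 3.
; Death loads or creates a ScoreBoard_BP save and appends a hard-coded placeholder name, with debug prints.
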(fn `Take_Damage`
  (params (Damage_to_Be_Taken :type "Float (double-precision)") (ColliderUsed :type "PrimitiveComponent Object Reference") (WasAttackFullyCharged :type Boolean))
  (bind _health (`self.Health`))
  (bind _stage3health (`self.Stage3Health`))
  (bind _saveinstance (`self.saveInstance`))
  (bind _phase (`self.Phase`))
  (bind _stage2health (`self.Stage2Health`))
  (bind _returnvalue (- Damage_to_Be_Taken (* (/ Damage_to_Be_Taken 100.0) (`self.Damage_Resistance`))))
  (bind _returnvalue_2 (* (`self.CriticalDamageMod`) _returnvalue))
  ;[1 1 1] PlayerDamage
  (`KismetSystemLibrary.PrintString` (`KismetStringLibrary.Conv_DoubleToString` _returnvalue_2))
  (if (not (`self.Dead`))
    (if (`KismetMathLibrary.BooleanNAND` WasAttackFullyCharged (`KismetStringLibrary.EqualEqual_StrStr` (`KismetSystemLibrary.GetObjectName` ColliderUsed) "Crit"))
      (set `self.Health` (- _health _returnvalue))
      (else
        (set `self.Health` (- _health _returnvalue_2))))
    (if (<= (`self.Health`) 0.0)
      (if (== _phase 3)
        (set `self.Dead` true)
        (bind _returnvalue_3 (`GameplayStatics.DoesSaveGameExist` (`self.Slot Name`) (`self.User Index`)))
        (if _returnvalue_3
          (bind _returnvalue_4 (`GameplayStatics.LoadGameFromSlot` (`self.Slot Name`) (`self.User Index`)))
          (bind _asscore_board_bp (cast `/Game/BloodRift/LevelDesign/ScoreBoard_BP` _returnvalue_4))
          (set `self.saveInstance` _asscore_board_bp)
          (else
            (bind _returnvalue_5 (`GameplayStatics.CreateSaveGameObject` "/Game/BloodRift/LevelDesign/ScoreBoard_BP.ScoreBoard_BP_C"))
            (set `self.saveInstance` _returnvalue_5)))
        (`KismetArrayLibrary.Array_Add` (`/Game/BloodRift/LevelDesign/ScoreBoard_BP.name` _saveinstance) "bob")
        (`GameplayStatics.SaveGameToSlot` _saveinstance (`self.Slot Name`) (`self.User Index`))
        (for _array_element (`/Game/BloodRift/LevelDesign/ScoreBoard_BP.name` (`self.saveInstance`))
          (`KismetSystemLibrary.PrintString` _array_element))
        (else
          (`/Engine/EditorBlueprintResources/StandardMacros.IncrementInt` _phase
            (:`  `
              (switch `int` (- _phase 2)
                (:`0`
                  (set `self.MaxHealth` _stage2health)
                  (set `self.Health` _stage2health))
                (:`1`
                  (set `self.MaxHealth` _stage3health)
                  (set `self.Health` _stage3health))))))))))

(fn `UserConstructionScript`)