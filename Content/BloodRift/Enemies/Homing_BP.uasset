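; Enemy homing projectile that damages the player on box overlap and then destroys itself.
; After a brief one-time delay, Tick turns it toward the player and lerps its position closer until it is within a set range.
; Outside homing it flies straight along its forward vector, so the final approach can be dodged.
; Movement uses frame-rate-dependent per-tick lerps without sweep, and the actor expires after a few seconds.
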(event `self.ReceiveTick`
  (params (DeltaSeconds :type "Float (single-precision)"))
  (bind _returnvalue (`self.K2_GetActorLocation`))
  (`|ExecutionSequence`
    (:`then_0`
      (`/Engine/EditorBlueprintResources/StandardMacros.DoOnce` false
        (:`Completed`
          (`KismetSystemLibrary.Delay` 0.2)
          (set `self.Home_In?` true))))
    (:`then_1`
      (`|ExecutionSequence`
        (:`then_0`
          (if (`self.Home_In?`)
            (`self.K2_SetActorRotation` (`KismetMathLibrary.FindLookAtRotation` (`self.K2_GetActorLocation`) (`self.K2_GetActorLocation` (`GameplayStatics.GetPlayerCharacter` 0))))
            (if (> (`self.GetDistanceTo` (`GameplayStatics.GetPlayerCharacter` 0)) 1250.0)
              (`self.K2_SetActorLocation` (`KismetMathLibrary.VLerp` (`self.K2_GetActorLocation`) (`self.K2_GetActorLocation` (`GameplayStatics.GetPlayerCharacter` 0)) 0.08))
              (else
                (set `self.Home_In?` false)))
            (else
              (`self.K2_SetActorLocation` (`KismetMathLibrary.VLerp` _returnvalue (+ (* (`KismetMathLibrary.GetForwardVector` (`self.K2_GetActorRotation`)) 600.0) _returnvalue) 0.08)))))
        (:`then_1`
          (`KismetSystemLibrary.Delay` 4.0)
          (`self.K2_DestroyActor`))))))

(event `self.Box.OnComponentBeginOverlap`
  (params (OverlappedComponent :type "PrimitiveComponent Object Reference") (OtherActor :type "Actor Object Reference") (OtherComp :type "PrimitiveComponent Object Reference") (OtherBodyIndex :type Integer) (bFromSweep :type Boolean) (SweepResult :type "HitResult Structure (by ref)"))
  (if (== (`GameplayStatics.GetObjectClass` OtherActor) "/Game/BloodRift/Character/Player.Player_C")
    (bind _asplayer (cast `/Game/BloodRift/Character/Player` OtherActor))
    (`/Game/BloodRift/Character/Player.TakeDamage` _asplayer (`self.Damage`))
    (`self.K2_DestroyActor`)))

(fn `UserConstructionScript`)