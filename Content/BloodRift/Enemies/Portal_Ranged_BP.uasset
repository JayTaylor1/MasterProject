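; Enemy portal actor that spawns Ranged_BP enemies one at a time at its SpawnPoint, up to a SpawnAmount limit.
; Tick uses a Spawn flag and a DoOnce to spawn each enemy, then re-arms once the tracked SpawnedEnemy is no longer valid.
; The portal destroys itself on the tick after AmountSpawned reaches the limit, without waiting for the last enemy to die.
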(event `self.ReceiveTick`
  (params (DeltaSeconds :type "Float (single-precision)"))
  (if (< (`self.Amount_Spawned`) (`self.Spawn_Amount`))
    (if (`self.Spawn?`)
      (`/Engine/EditorBlueprintResources/StandardMacros.DoOnce` false :!label _label
        (:`Completed`
          (bind _returnvalue (`|SpawnActorFromClass` "/Game/BloodRift/Enemies/Ranged_BP.Ranged_BP_C" (`KismetMathLibrary.MakeTransform` (`SceneComponent.K2_GetComponentLocation` (`self.Spawn_Point`))) "Undefined" "OverrideRootScale" null null))
          (set `self.Spawned_Enemy` _returnvalue)
          (set `self.Spawn?` false)
          (`/Engine/EditorBlueprintResources/StandardMacros.IncrementInt` (`self.Amount_Spawned`))))
      (else
        (`|ExecutionSequence`
          (:`then_0`
            (goto _label :!via `Reset`))
          (:`then_1`
            (if (`KismetSystemLibrary.IsValid` (`self.Spawned_Enemy`))
              _
              (elif (< (`self.Amount_Spawned`) (`self.Spawn_Amount`))
                (set `self.Spawn?` true)
                (else
                  (`self.K2_DestroyActor`))))))))
    (else
      (`self.K2_DestroyActor`))))

(fn `UserConstructionScript`)