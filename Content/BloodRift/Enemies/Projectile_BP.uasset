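; Enemy projectile that flies forward or homes in on the player, dealing damage on overlap.
; Tick drives movement: homing missiles fly straight briefly, track the player, then stop homing at close range.
; Non-homing shots advance once InFlight is set, with a timer event re-aligning Scene to SpawnPoint's rotation.
; It destroys itself after a lifetime delay or on overlapping the player or any non-ignored class.
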(event `self.ReceiveTick`
  (params (DeltaSeconds :type "Float (single-precision)"))
  (`/Engine/EditorBlueprintResources/StandardMacros.IsValid` (`self.Scene`)
    (:`Is Valid`
      (`|ExecutionSequence`
        (:`then_0`
          (if (`self.HomingMissile`)
            (`|ExecutionSequence`
              (:`then_0`
                (`/Engine/EditorBlueprintResources/StandardMacros.DoOnce` false
                  (:`Completed`
                    (`KismetSystemLibrary.Delay` 0.2)
                    (set `self.Home in?` true))))
              (:`then_1`
                (if (not (`self.Home in?`))
                  (`self.K2_SetActorLocation` (`KismetMathLibrary.VLerp` (`self.K2_GetActorLocation`) (+ (* (`KismetMathLibrary.GetForwardVector` (`self.K2_GetActorRotation`)) 600.0) (`self.K2_GetActorLocation`)) (`self.FlightAlpha`)) :!label _label)
                  (else
                    (`self.K2_SetActorRotation` (`KismetMathLibrary.FindLookAtRotation` (`self.K2_GetActorLocation`) (`self.K2_GetActorLocation` (`GameplayStatics.GetPlayerCharacter` 0))))
                    (if (> (`self.GetDistanceTo` (`GameplayStatics.GetPlayerCharacter` 0)) 1250.0)
                      (`self.K2_SetActorLocation` (`KismetMathLibrary.VLerp` (`self.K2_GetActorLocation`) (`self.K2_GetActorLocation` (`GameplayStatics.GetPlayerCharacter` 0)) (* (`self.FlightAlpha`) 0.6)))
                      (else
                        (set `self.Home in?` false)))))))
            (elif (`self.In_Flight`)
              (`|ExecutionSequence`
                (:`then_0`
                  (goto _label))
                (:`then_1`
                  (if (not (`KismetSystemLibrary.K2_IsTimerActiveHandle` (`self.CacheTimer`)))
                    (bind _returnvalue (`KismetSystemLibrary.K2_SetTimerDelegate` (`|CreateDelegate` :!event `ChangeRot`) (* (`self.FlightAlpha`) 0.6)))
                    (set `self.CacheTimer` _returnvalue)))))))
        (:`then_1`
          (`KismetSystemLibrary.Delay` 10.0)
          (`self.K2_DestroyActor`))))))

(event `ChangeRot`
  (bind _scene (`self.Scene`))
  ;[1 1 1] Change Rot Timed Event
  (`/Engine/EditorBlueprintResources/StandardMacros.IsValid` _scene
    (:`Is Valid`
      (`SceneComponent.K2_SetWorldRotation` _scene (`SceneComponent.K2_GetComponentRotation` (`self.SpawnPoint`)) false false)
      (`KismetSystemLibrary.K2_ClearAndInvalidateTimerHandle` (`self.CacheTimer`)))))

(event `self.Box.OnComponentBeginOverlap`
  (params (OverlappedComponent :type "PrimitiveComponent Object Reference") (OtherActor :type "Actor Object Reference") (OtherComp :type "PrimitiveComponent Object Reference") (OtherBodyIndex :type Integer) (bFromSweep :type Boolean) (SweepResult :type "HitResult Structure (by ref)"))
  ;[1 1 1] Collision
  (if (not (== OtherActor (`GameplayStatics.GetPlayerCharacter` 0)))
    (if (not (`KismetArrayLibrary.Array_Contains` (`self.Ignorables`) (`GameplayStatics.GetObjectClass` OtherActor)))
      (`self.K2_DestroyActor` :!label _label_2))
    (else
      (bind _asplayer (cast `/Game/BloodRift/Character/Player` OtherActor))
      (`/Game/BloodRift/Character/Player.TakeDamage` _asplayer (`self.Damage`))
      (goto _label_2))))

(fn `StartFlight`
  (locals (StartPosition :type "Vector Structure"))
  (set `self.In_Flight` true))

(fn `UserConstructionScript`)