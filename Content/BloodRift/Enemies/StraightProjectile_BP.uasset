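; Straight-flying enemy projectile that damages the Player when its Box overlaps them.
; Once StartFlight sets InFlight, Tick sweeps it along its forward vector by a fixed, frame-rate-dependent step.
; A short re-armed timer appears to drive ChangeRot, copying the SpawnPoint's rotation onto Scene.
; A Delay on Tick destroys the actor after a few seconds, whether launched or not.
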(event `ChangeRot`
  (`SceneComponent.K2_SetWorldRotation` (`self.Scene`) (`SceneComponent.K2_GetComponentRotation` (`self.SpawnPoint`)) false false)
  (`KismetSystemLibrary.K2_ClearAndInvalidateTimerHandle` (`self.CacheTimer`)))

(event `self.ReceiveTick`
  (params (DeltaSeconds :type "Float (single-precision)"))
  (bind _returnvalue (`self.K2_GetActorLocation`))
  (`|ExecutionSequence`
    (:`then_0`
      (if (`self.In_Flight`)
        (`|ExecutionSequence`
          (:`then_0`
            (`self.K2_SetActorLocation` (`KismetMathLibrary.VLerp` _returnvalue (+ (* (`KismetMathLibrary.GetForwardVector` (`self.K2_GetActorRotation`)) 600.0) _returnvalue) 0.1) true))
          (:`then_1`
            (if (not (`KismetSystemLibrary.K2_IsTimerActiveHandle` (`self.CacheTimer`)))
              (bind _returnvalue_2 (`KismetSystemLibrary.K2_SetTimerDelegate` (`|CreateDelegate` :!event `ChangeRot`) 0.06))
              (set `self.CacheTimer` _returnvalue_2))))))
    (:`then_1`
      (`KismetSystemLibrary.Delay` 4.0)
      (`self.K2_DestroyActor`))))

(event `self.Box.OnComponentBeginOverlap`
  (params (OverlappedComponent :type "PrimitiveComponent Object Reference") (OtherActor :type "Actor Object Reference") (OtherComp :type "PrimitiveComponent Object Reference") (OtherBodyIndex :type Integer) (bFromSweep :type Boolean) (SweepResult :type "HitResult Structure (by ref)"))
  (if (== (`GameplayStatics.GetObjectClass` OtherActor) "/Game/BloodRift/Character/Player.Player_C")
    (bind _asplayer (cast `/Game/BloodRift/Character/Player` OtherActor))
    (`/Game/BloodRift/Character/Player.TakeDamage` _asplayer (`self.Damage`))))

(fn `StartFlight`
  (locals (StartPosition :type "Vector Structure"))
  (set `self.In_Flight` true))

(fn `UserConstructionScript`)