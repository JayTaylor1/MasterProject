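; ItemClassBase_BP is the base pickup item, which Interact moves into the player's inventory.
; Consumables merge stacks with matching Consumable slots or inventory entries, then expire via a short lifespan, with a Gate controlling fallback to placement.
; Placed items take the first empty inventory slot, attach to the player's Sphere, hide with collision off and refresh the inventory widget.
; Helpers restore visibility and collision or colour the cube by rarity.
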(event `/Game/BloodRift/Character/InteractInterface.interact`
  (params (Player :type "/Game/BloodRift/Character/Player Object Reference"))
  (bind _inventory (`/Game/BloodRift/Character/Player.Inventory` Player))
  (bind _consumable1 (`/Game/BloodRift/Character/Player.Consumable1` Player))
  (bind _inventorywidget (`/Game/BloodRift/Character/Player.InventoryWIdget` Player))
  (bind _consumable2 (`/Game/BloodRift/Character/Player.Consumable2` Player))
  (bind _returnvalue (`GameplayStatics.GetObjectClass` self))
  (bind _returnvalue_2 (`KismetMathLibrary.ClassIsChildOf` _returnvalue "/Game/BloodRift/Items/Consumable/Consumable.Consumable_C"))
  (if _returnvalue_2
    (`/Engine/EditorBlueprintResources/StandardMacros.IsValid` _consumable1
      (:`Is Valid`
        (if (== _returnvalue (`GameplayStatics.GetObjectClass` _consumable1))
          (bind _asconsumable (cast `/Game/BloodRift/Items/Consumable/Consumable` self))
          (bind _asconsumable_2 (cast `/Game/BloodRift/Items/Consumable/Consumable` _consumable1))
          (set `/Game/BloodRift/Items/Consumable/Consumable.stacks` (+ (`/Game/BloodRift/Items/Consumable/Consumable.stacks` _asconsumable_2) (`/Game/BloodRift/Items/Consumable/Consumable.stacks` _asconsumable)) _asconsumable_2)
          (`/Game/BloodRift/Items/Equipment/Inventory.Consumable1UpdateStacks` _inventorywidget)
          (`self.SetLifeSpan` 0.001)
          (else
            (`/Engine/EditorBlueprintResources/StandardMacros.IsValid` _consumable2 :!label _label
              (:`Is Valid`
                (if (== _returnvalue (`GameplayStatics.GetObjectClass` _consumable2))
                  (bind _asconsumable_3 (cast `/Game/BloodRift/Items/Consumable/Consumable` self))
                  (bind _asconsumable_4 (cast `/Game/BloodRift/Items/Consumable/Consumable` _consumable2))
                  (set `/Game/BloodRift/Items/Consumable/Consumable.stacks` (+ (`/Game/BloodRift/Items/Consumable/Consumable.stacks` _asconsumable_4) (`/Game/BloodRift/Items/Consumable/Consumable.stacks` _asconsumable_3)) _asconsumable_4)
                  (`/Game/BloodRift/Items/Equipment/Inventory.Consumable2UpdateStacks` _inventorywidget)
                  (`self.SetLifeSpan` 0.001)
                  (else
                    (for (_array_element _array_index) _inventory :!label _label_2
                      (`/Engine/EditorBlueprintResources/StandardMacros.IsValid` _array_element
                        (:`Is Not Valid`
                          (`KismetArrayLibrary.Array_Set` _inventory _array_index self)
                          (`self.K2_AttachToComponent` (`/Game/BloodRift/Character/Player.Sphere` Player) "None" "SnapToTarget" "SnapToTarget" "SnapToTarget")
                          (`self.HideItem`)
                          (`/Game/BloodRift/Items/Equipment/Inventory.InventoryLoad` (`/Game/BloodRift/Character/Player.InventoryWIdget` Player) _array_index)
                          (break)))))))
              (:`Is Not Valid`
                (for (_array_element_2 _array_index_2) _inventory
                  (`/Engine/EditorBlueprintResources/StandardMacros.IsValid` _array_element_2
                    (:`Is Valid`
                      (if _returnvalue_2
                        (if (== _returnvalue (`GameplayStatics.GetObjectClass` _array_element_2))
                          (bind _asconsumable_5 (cast `/Game/BloodRift/Items/Consumable/Consumable` self))
                          (bind _asconsumable_6 (cast `/Game/BloodRift/Items/Consumable/Consumable` _array_element_2))
                          (set `/Game/BloodRift/Items/Consumable/Consumable.stacks` (+ (`/Game/BloodRift/Items/Consumable/Consumable.stacks` _asconsumable_6) (`/Game/BloodRift/Items/Consumable/Consumable.stacks` _asconsumable_5)) _asconsumable_6)
                          (`/Game/BloodRift/Items/Equipment/Inventory.InventoryLoad` _inventorywidget _array_index_2)
                          (`self.SetLifeSpan` 0.01)
                          (goto _label_3 :!via `Close`))))))
                (`/Engine/EditorBlueprintResources/StandardMacros.Gate` false :!label _label_3
                  (:`Exit`
                    (goto _label_2))))))))
      (:`Is Not Valid`
        (goto _label)))
    (else
      (goto _label_2))))

(fn `CubeColourChange`
  (bind _itemrarity (`self.ItemRarity`))
  (bind _cube (`self.Cube`))
  (if (`KismetStringLibrary.EqualEqual_StrStr` _itemrarity "Mundane")
    (`PrimitiveComponent.SetMaterial` _cube 0 "/Game/BloodRift/Spells/Colour/White.White")
    (elif (`KismetStringLibrary.EqualEqual_StrStr` _itemrarity "Common")
      (`PrimitiveComponent.SetMaterial` _cube 0 "/Game/BloodRift/Spells/Colour/Green.Green")
      (elif (`KismetStringLibrary.EqualEqual_StrStr` _itemrarity "Rare")
        (`PrimitiveComponent.SetMaterial` _cube 0 "/Game/BloodRift/Spells/Colour/Blue.Blue")
        (elif (`KismetStringLibrary.EqualEqual_StrStr` _itemrarity "Epic")
          (`PrimitiveComponent.SetMaterial` _cube 0 "/Game/BloodRift/Spells/Colour/Purple.Purple")
          (elif (`KismetStringLibrary.EqualEqual_StrStr` _itemrarity "Legendary")
            (`PrimitiveComponent.SetMaterial` _cube 0 "/Game/BloodRift/Spells/Colour/Orange.Orange")))))))

(fn `HideItem`
  (`SceneComponent.SetHiddenInGame` (`self.Cube`) true false)
  (`self.SetActorEnableCollision` self false)
  (`PrimitiveComponent.SetCollisionEnabled` (`self.collision`) "NoCollision"))

(fn `UnHide`
  (`SceneComponent.SetHiddenInGame` (`self.Cube`) false false)
  (`self.SetActorEnableCollision` true)
  (`PrimitiveComponent.SetCollisionEnabled` (`self.collision`) "QueryOnly"))

(fn `UserConstructionScript`)