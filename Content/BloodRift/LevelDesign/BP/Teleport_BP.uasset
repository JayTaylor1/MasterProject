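; Paired teleporter pad that moves the player to the actor referenced by Link when they overlap InteractRange.
; It sets the destination's Lock to prevent an immediate bounce back; each pad clears its own Lock when the player leaves.
; A successful teleport puts every Teleport_BP in the level on a shared ten-second cooldown, checked through Link, with meshes turned red until it ends and they return to blue.
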(event `self.InteractRange.OnComponentBeginOverlap`
  (params (OverlappedComponent :type "PrimitiveComponent Object Reference") (OtherActor :type "Actor Object Reference") (OtherComp :type "PrimitiveComponent Object Reference") (OtherBodyIndex :type Integer) (bFromSweep :type Boolean) (SweepResult :type "HitResult Structure (by ref)"))
  (bind _link (`self.Link`))
  (cast `/Game/BloodRift/Character/Player` OtherActor)
  (if (not (`self.Lock`))
    (set `/Game/BloodRift/LevelDesign/BP/Teleport_BP.Lock` true _link)
    (if (not (`/Game/BloodRift/LevelDesign/BP/Teleport_BP.CoolDown` (`self.Link`)))
      (`self.K2_SetActorLocation` (`GameplayStatics.GetPlayerPawn` 0) (`self.K2_GetActorLocation` _link) false false)
      (bind _outactors (`GameplayStatics.GetAllActorsOfClass` "Teleport_BP_C"))
      (for _array_element _outactors
        (set `/Game/BloodRift/LevelDesign/BP/Teleport_BP.CoolDown` true _array_element)
        (`PrimitiveComponent.SetMaterial` (`/Game/BloodRift/LevelDesign/BP/Teleport_BP.StaticMesh` _array_element) 0 "/Game/BloodRift/Spells/Colour/Red.Red"))
      (`KismetSystemLibrary.Delay` 10.0)
      (for _array_element_2 _outactors
        (set `/Game/BloodRift/LevelDesign/BP/Teleport_BP.CoolDown` false _array_element_2)
        (`PrimitiveComponent.SetMaterial` (`/Game/BloodRift/LevelDesign/BP/Teleport_BP.StaticMesh` _array_element_2) 0 "/Game/BloodRift/Spells/Colour/Blue.Blue")))))

(event `self.InteractRange.OnComponentEndOverlap`
  (params (OverlappedComponent :type "PrimitiveComponent Object Reference") (OtherActor :type "Actor Object Reference") (OtherComp :type "PrimitiveComponent Object Reference") (OtherBodyIndex :type Integer))
  (cast `/Game/BloodRift/Character/Player` OtherActor)
  (set `self.Lock` false))

(fn `UserConstructionScript`)