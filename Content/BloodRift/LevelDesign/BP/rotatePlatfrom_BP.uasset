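; Level-design rotating platform that moves its Cone component in a horizontal circle around a Center actor at its own Distance.
; Tick advances the angle by a per-frame AngularVelocity and places the cone with degree-based sine and cosine.
; AlignNew selects another platform by signed Distance difference and speeds it up tenfold until their angles nearly match, then its Tick restores the speed.
; Player attachment logic exists but is unconnected.
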(event `self.ReceiveTick`
  (params (DeltaSeconds :type "Float (single-precision)"))
  (bind _returnvalue (`self.GetTransform`))
  (bind _angle (`self.angle`))
  (bind _distance (`self.distance`))
  (bind _returnvalue_2 (`self.GetTransform` (`self.center`)))
  (`SceneComponent.K2_SetWorldTransform` (`self.Cone`) (`KismetMathLibrary.MakeTransform` (`KismetMathLibrary.MakeVector` (+ (* (`KismetMathLibrary.DegCos` _angle) _distance) (.x (.location _returnvalue_2))) (+ (.y (.location _returnvalue_2)) (* _distance (`KismetMathLibrary.DegSin` _angle))) (.z (.location _returnvalue))) (.rotation _returnvalue) (.scale _returnvalue)) false false)
  (if (`self.check`)
    (if (`KismetMathLibrary.NearlyEqual_FloatFloat` (`/Game/BloodRift/LevelDesign/BP/rotatePlatfrom_BP.angle` (`self.other`)) (`self.angle`) 10.0)
      (`self.speedDown`)
      (set `self.check` false)))
  (set `self.angle` (+ _angle (`self.angularVelocity`)))
  (if (> _angle 360.0)
    (set `self.angle` 0.0)))

(fn `alignNew`
  (bind _other (`self.other`))
  (bind _outactors (`GameplayStatics.GetAllActorsOfClass` "rotatePlatfrom_BP_C"))
  (for _array_element _outactors
    (if (not (== self _array_element))
      (bind _returnvalue (- (`/Game/BloodRift/LevelDesign/BP/rotatePlatfrom_BP.distance` _array_element) (`self.distance`)))
      (if (> (`self.temp`) _returnvalue)
        (set `self.temp` _returnvalue)
        (set `self.other` _array_element))))
  (set `/Game/BloodRift/LevelDesign/BP/rotatePlatfrom_BP.other` self _other)
  (set `/Game/BloodRift/LevelDesign/BP/rotatePlatfrom_BP.check` true _other)
  (`self.speedUp` _other))

(fn `speedDown`
  (set `self.angularVelocity` (/ (`self.angularVelocity`) 10.0)))

(fn `speedUp`
  (set `self.angularVelocity` (* (`self.angularVelocity`) 10.0)))

(fn `UserConstructionScript`)